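; Powser character for a board game, taking a two-phase targeting turn driven by move and confirm events from its W_Roll widget.
; Phase one teleports it between linked left/right spaces; confirming tilts the camera down for phase two.
; Phase two slides a three-space highlight through the current space's range, with index rollover for wrapping.
; Confirming again resets untargeted spaces' materials and signals turn end.
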(event `self.ReceiveBeginPlay`
  (bind _returnvalue (`GameplayStatics.GetPlayerController` 0))
  (bind _asw_roll (cast `/Game/W_Roll` (`WidgetComponent.GetWidget` (`self.W_Roll`))))
  (bind _output_get (set `self.As W Powser` _asw_roll))
  (`Widget.SetVisibility` _output_get "Hidden")
  (`self.EnableInput` _returnvalue)
  (`EnhancedInputSubsystemInterface.AddMappingContext` (pcsubsystem `EnhancedInputLocalPlayerSubsystem` _returnvalue) "/Game/ThirdPerson/Input/IMC_Default.IMC_Default" 0 (struct))
  (`self.OnSetupEnded`))

(event `OnConfirm`
  (bind _turnstep (`self.TurnStep`))
  (if (== _turnstep 1)
    (`self.StartPhase2`)
    (elif (== _turnstep 2)
      (`self.EndPowserTurn`))))

(event `OnTurn`
  (bind _as_w_powser (`self.As W Powser`))
  (set `self.TurnStep` 1)
  (`PlayerController.SetViewTargetWithBlend` (`GameplayStatics.GetPlayerController` 0) self 0.0 "VTBlend_Linear" 0.0 false)
  (`/Game/BP_PowserSpace.SetHighlighted` (`self.CurrentSpace`) true)
  (add `/Game/W_Roll.OnMovePressed` _as_w_powser (delegate `OnMove`))
  (add `/Game/W_Roll.OnConfirmPressed` _as_w_powser (delegate `OnConfirm`)))

(event `OnLeftPressed`
  (if (== (`self.TurnStep`) 1)
    (`self.MoveToSpace` (`/Game/BP_PowserSpace.SpaceLeft` (`self.CurrentSpace`)))
    (elif (== (`self.TurnStep`) 2)
      (`self.ChangeBoardSpacesSelected` -1))))

(event `OnMove`
  (params (Value :type "Vector2D Structure"))
  (bind _x (`KismetMathLibrary.BreakVector2D` Value))
  (if (< _x 0.0)
    (`self.OnLeftPressed`)
    (elif (> _x 0.0)
      (`self.OnRightPressed`))))

(event `EndPowserTurn`
  (for _array_element (`/Game/BP_PowserSpace.SpacesInRange` (`self.CurrentSpace`))
    (if (not (`/Game/BP_BoardSpace.Targeted` _array_element))
      (`/Game/BP_BoardSpace.ResetMaterial` _array_element)))
  (set `self.TurnStep` 0)
  (`self.OnPowserTurnEnded`))

(event `MoveToSpace`
  (params (NewSpace :type "/Game/BP_PowserSpace Object Reference"))
  (`self.K2_SetActorLocation` (`self.K2_GetActorLocation` NewSpace) false true)
  (`/Game/BP_PowserSpace.SetHighlighted` (`self.CurrentSpace`) false)
  (bind _output_get (set `self.CurrentSpace` NewSpace))
  (`/Game/BP_PowserSpace.SetHighlighted` _output_get true))

(event `StartPhase2`
  (set `self.TurnStep` 2)
  (`SceneComponent.K2_SetRelativeRotation` (`self.SpringArm`) (struct :`Pitch` -80.0) false false)
  (`self.UpdateSpacesSelected`))

(event `OnRightPressed`
  (if (== (`self.TurnStep`) 1)
    (`self.MoveToSpace` (`/Game/BP_PowserSpace.SpaceRight` (`self.CurrentSpace`)))
    (elif (== (`self.TurnStep`) 2)
      (`self.ChangeBoardSpacesSelected` 1))))

(event `ChangeBoardSpacesSelected`
  (params (ChangeBy :type Integer))
  (bind _returnnum (`self.ChangeByWithRollover` (`self.SpaceSelectIndex`) ChangeBy (`KismetArrayLibrary.Array_LastIndex` (`/Game/BP_PowserSpace.SpacesInRange` (`self.CurrentSpace`)))))
  (`KismetSystemLibrary.PrintString` (`KismetStringLibrary.Conv_IntToString` _returnnum))
  (set `self.SpaceSelectIndex` _returnnum)
  (`self.UpdateSpacesSelected`))

(fn `AddCoins`
  (params (Number :type Integer))
  (set `self.Coins` (+ (`self.Coins`) Number)))

(fn `ChangeByWithRollover`
  (params (Index :type Integer) (ChangeBy :type Integer) (ListLength :type Integer))
  (returns (ReturnNum :type Integer))
  (bind _returnvalue (+ Index ChangeBy))
  (if (>= _returnvalue 0)
    (if (<= _returnvalue ListLength)
      (return _returnvalue)
      (else
        (return 0)))
    (else
      (return ListLength))))

(fn `UpdateSpacesSelected`
  (bind _spacesinrange (`/Game/BP_PowserSpace.SpacesInRange` (`self.CurrentSpace`)))
  (for _array_element (`/Game/BP_PowserSpace.SpacesInRange` (`self.CurrentSpace`))
    (`/Game/BP_BoardSpace.SetMatTo` _array_element "/Game/M_BoardSpace_Inst4.M_BoardSpace_Inst4")
    (set `/Game/BP_BoardSpace.Targeted` false _array_element))
  (for _index (range -1 2)
    (if (`/Game/BP_PowserSpace.SpacesWrap` (`self.CurrentSpace`))
      (bind _returnnum (`self.ChangeByWithRollover` (`self.SpaceSelectIndex`) _index (`KismetArrayLibrary.Array_LastIndex` _spacesinrange)))
      (bind _output (`|GetArrayItem` _spacesinrange _returnnum))
      (`/Game/BP_BoardSpace.SetMatTo` _output "/Game/M_BoardSpace_Inst5.M_BoardSpace_Inst5")
      (else
        (bind _output_2 (`|GetArrayItem` _spacesinrange (+ _index (`self.SpaceSelectIndex`))))
        (if (`KismetSystemLibrary.IsValid` _output_2)
          (`/Game/BP_BoardSpace.SetMatTo` _output_2 "/Game/M_BoardSpace_Inst5.M_BoardSpace_Inst5")
          (set `/Game/BP_BoardSpace.Targeted` true _output))))))

(fn `UserConstructionScript`)