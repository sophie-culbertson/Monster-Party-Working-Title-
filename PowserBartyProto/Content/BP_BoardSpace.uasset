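; Board space actor for a Mario Party-style board game, with a space type (Blue, Red, Green, Bowser or Star) and branch arrows for crossroads.
; The construction script picks the cylinder material from the type and caches it; SetMatTo overrides it and ResetMaterial reapplies the type's material.
; Arrows start hidden, SetArrowVisibility toggles them, and ChangeArrowSelected cycles the selection with wraparound, updating each arrow's material to mark the selected one.
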(event `self.ReceiveBeginPlay`
  (set `self.AtCrossroads` false)
  (if (`KismetArrayLibrary.Array_IsNotEmpty` (`self.Arrows`))
    (set `self.ArrowSelected` 0)
    (`self.SetArrowVisibility` false)))

(event `ChangeArrowSelected`
  (params (Amount :type Integer))
  (bind _returnvalue (+ Amount (`self.ArrowSelected`)))
  (bind _returnvalue_2 (- (`KismetArrayLibrary.Array_Length` (`self.Arrows`)) 1))
  (if (< _returnvalue 0)
    (set `self.ArrowSelected` _returnvalue_2)
    (elif (> _returnvalue _returnvalue_2)
      (set `self.ArrowSelected` 0)
      (else
        (set `self.ArrowSelected` _returnvalue))))
  (for (_array_element _array_index) (`self.Arrows`)
    (`/Game/BP_Arrow.SetMaterial` _array_element (== _array_index (`self.ArrowSelected`)))))

(event `SetArrowVisibility`
  (params (visibility :type Boolean))
  (for _array_element (`self.Arrows`)
    (`/Game/BP_Arrow.SetVisibility` _array_element visibility)))

(event `SetMatTo`
  (params (mat :type "MaterialInterface Object Reference"))
  (`PrimitiveComponent.SetMaterial` (`self.Cylinder`) 0 mat))

(fn `ResetMaterial`
  (bind _returnvalue (select `/Game/ESpaceType` (`self.SpaceType`) :`NewEnumerator0` "/Game/M_BoardSpace_Inst.M_BoardSpace_Inst" :`NewEnumerator1` "/Game/M_BoardSpace_Inst1.M_BoardSpace_Inst1" :`NewEnumerator2` "/Game/M_BoardSpace_Inst2.M_BoardSpace_Inst2" :`NewEnumerator3` "/Game/M_BoardSpace_Inst1.M_BoardSpace_Inst1" :`NewEnumerator4` "/Game/M_BoardSpace_Inst3.M_BoardSpace_Inst3" :!type "MaterialInterface Object Reference"))
  (`PrimitiveComponent.SetMaterial` (`self.Cylinder`) 0 _returnvalue)
  (set `self.DefaultMat` _returnvalue))

(fn `UserConstructionScript`
  (bind _returnvalue (select `/Game/ESpaceType` (`self.SpaceType`) :`NewEnumerator0` "/Game/M_BoardSpace_Inst.M_BoardSpace_Inst" :`NewEnumerator1` "/Game/M_BoardSpace_Inst1.M_BoardSpace_Inst1" :`NewEnumerator2` "/Game/M_BoardSpace_Inst2.M_BoardSpace_Inst2" :`NewEnumerator3` "/Game/M_BoardSpace_Inst1.M_BoardSpace_Inst1" :`NewEnumerator4` "/Game/M_BoardSpace_Inst3.M_BoardSpace_Inst3" :!type "MaterialInterface Object Reference"))
  (`PrimitiveComponent.SetMaterial` (`self.Cylinder`) 0 _returnvalue)
  (set `self.DefaultMat` _returnvalue))