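; Board-game player character that takes a turn by rolling dice and walking along linked spaces.
; The W_Roll widget supplies the roll result and move and confirm inputs, bound per turn.
; AI MoveTo hops space to space, counting down moves and pausing at crossroads for an arrow-based path choice.
; When moves run out, it unbinds the widget, adjusts coins for Blue or Red spaces, and fires turn-ended and coin-collected dispatchers.
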(event `self.ReceiveBeginPlay`
  (bind _returnvalue (`GameplayStatics.GetPlayerController` 0))
  (bind _asw_roll (cast `/Game/W_Roll` (`WidgetComponent.GetWidget` (`self.W_Roll`))))
  (bind _output_get (set `self.As W Roll` _asw_roll))
  (`Widget.SetVisibility` _output_get "Hidden")
  (`self.EnableInput` _returnvalue)
  (`EnhancedInputSubsystemInterface.AddMappingContext` (pcsubsystem `EnhancedInputLocalPlayerSubsystem` _returnvalue) "/Game/ThirdPerson/Input/IMC_Default.IMC_Default" 0 (struct)))

(event `RollDice`
  (bind _as_w_roll (`self.As W Roll`))
  (bind _as_w_roll_2 (`self.As W Roll`))
  (add `/Game/W_Roll.OnMovePressed` _as_w_roll (delegate `OnMove`))
  (add `/Game/W_Roll.OnConfirmPressed` _as_w_roll (delegate `OnConfirmPressed`))
  (`PlayerController.SetViewTargetWithBlend` (`GameplayStatics.GetPlayerController` 0) self 0.0 "VTBlend_Linear" 0.0 false)
  (`/Game/W_Roll.StartRoll` _as_w_roll_2)
  (add `/Game/W_Roll.OnRollStopped` _as_w_roll_2 (delegate `RollStopped`))
  (`Widget.SetVisibility` _as_w_roll_2 "Visible"))

(event `RollStopped`
  (params (Number :type Integer))
  (set `self.MovesRemaining` Number)
  (`self.MoveToSpace` (`self.CurrentSpace`)))

(event `OnMove`
  (params (Value :type "Vector2D Structure"))
  (bind _x (`KismetMathLibrary.BreakVector2D` Value))
  (if (< _x 0.0)
    (`self.OnLeftPressed`)
    (elif (> _x 0.0)
      (`self.OnRightPressed`))))

(event `MoveToSpace`
  (params (CurrentSpace :type "/Game/BP_BoardSpace Object Reference") (NextSpaceIndex :type Integer))
  (`KismetSystemLibrary.PrintString` (`KismetSystemLibrary.GetDisplayName` CurrentSpace))
  (bind _output_get (set `self.CurrentSpace` (`|GetArrayItem` (`/Game/BP_BoardSpace.NextSpace` CurrentSpace) NextSpaceIndex)))
  (bind _movementresult (`|AIMoveTo` self (`self.K2_GetActorLocation` _output_get) null)
    (:`OnSuccess`
      (bind _result (`/Engine/EditorBlueprintResources/StandardMacros.DecrementInt` (`self.MovesRemaining`))
        (:`  `
          (`TextBlock.SetText` (`/Game/W_Roll.TXT_Number` (`self.As W Roll`)) (`KismetTextLibrary.Conv_IntToText` _result))
          (if (> _result 0)
            (if (> (`KismetArrayLibrary.Array_Length` (`/Game/BP_BoardSpace.NextSpace` (`self.CurrentSpace`))) 1)
              (`self.ChoosePath`)
              (else
                (`self.MoveToSpace` (`self.CurrentSpace`))))
            (else
              (`self.TurnEnded`))))))))

(event `OnLeftPressed`
  (if (`self.ChoosingPath`)
    (`/Game/BP_BoardSpace.ChangeArrowSelected` (`self.CurrentSpace`) -1)))

(event `TurnEnded`
  (bind _as_w_roll (`self.As W Roll`))
  (`|ExecutionSequence`
    (:`then_0`
      (clear `/Game/W_Roll.OnMovePressed` _as_w_roll))
    (:`then_1`
      (clear `/Game/W_Roll.OnRollStopped` _as_w_roll))
    (:`then_2`
      (clear `/Game/W_Roll.OnConfirmPressed` _as_w_roll)
      (set `Widget.Visibility` "Hidden" _as_w_roll)
      (`KismetSystemLibrary.Delay` 1.0)
      (`|ExecutionSequence`
        (:`then_0`
          (switch `/Game/ESpaceType` (`/Game/BP_BoardSpace.SpaceType` (`self.CurrentSpace`))
            (:`NewEnumerator0`
              (`self.AddCoins` 3))
            (:`NewEnumerator1`
              (`self.AddCoins` -3))))
        (:`then_1`
          (`self.OnTurnEnded`)
          (clear `self.OnTurnEnded`)
          (`self.OnCoinCollected`))))))

(event `OnRightPressed`
  (if (`self.ChoosingPath`)
    (`/Game/BP_BoardSpace.ChangeArrowSelected` (`self.CurrentSpace`) 1)))

(event `OnConfirmPressed`
  (bind _currentspace (`self.CurrentSpace`))
  (if (`self.ChoosingPath`)
    (`self.MoveToSpace` _currentspace (`/Game/BP_BoardSpace.ArrowSelected` _currentspace))))

(event `ChoosePath`
  (bind _currentspace (`self.CurrentSpace`))
  (set `self.ChoosingPath` true)
  (set `/Game/BP_BoardSpace.AtCrossroads` true _currentspace)
  (`/Game/BP_BoardSpace.SetArrowVisibility` _currentspace true)
  (`/Game/BP_BoardSpace.ChangeArrowSelected` _currentspace 0))

(fn `AddCoins`
  (params (Number :type Integer))
  (set `self.Coins` (+ (`self.Coins`) Number))
  (`/Game/W_Roll.GetCoins` (`self.As W Roll`) Number))

(fn `UserConstructionScript`)