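; Game mode for a board party game that runs turn-based rounds for four characters and a Powser character.
; BeginPlay spawns the characters, places them on the "Start"-tagged board space, fixes turn order and adds the HUD.
; Each round starts with Powser's turn, then turn-ended events step through a copied order, triggering each character's dice roll.
; An emptied queue decrements Rounds and begins another round after a delay, with no end-of-game check.
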(event `self.ReceiveBeginPlay`
  (bind _outactors (`GameplayStatics.GetAllActorsOfClassWithTag` "/Game/BP_BoardSpace.BP_BoardSpace_C" "Start"))
  (set `self.StartingSpace` (`|GetArrayItem` _outactors))
  (bind _returnvalue (`GameplayStatics.GetActorOfClass` "/Game/BP_PowserCharacter.BP_PowserCharacter_C"))
  (set `self.PowserCharacter` _returnvalue)
  (for _index (range 4)
    (bind _returnvalue_2 (`|SpawnActorFromClass` "/Game/BP_Character.BP_Character_C" (`KismetMathLibrary.Conv_VectorToTransform` (`|GetArrayItem` (`self.PlayerSpawns`) _index)) "Undefined" "MultiplyWithRoot" null null))
    (set `/Game/BP_Character.CurrentSpace` (`self.StartingSpace`) _returnvalue_2))
  (bind _outactors_2 (`GameplayStatics.GetAllActorsOfClass` "/Game/BP_Character.BP_Character_C"))
  (set `self.TurnOrder` _outactors_2)
  (`self.InitiateRound`)
  (bind _returnvalue_3 (`|CreateWidget` "/Game/UI/W_HUD.W_HUD_C"))
  (`UserWidget.AddToViewport` _returnvalue_3 0))

(event `EndRound`
  (`/Engine/EditorBlueprintResources/StandardMacros.DecrementInt` (`self.Rounds`)
    (:`  `
      (`KismetSystemLibrary.Delay` 3.0)
      (`self.InitiateRound`))))

(event `InitiateRound`
  (set `self.RoundOrder` (`self.TurnOrder`))
  (`self.StartTurnPowser`)
  (add `/Game/BP_PowserCharacter.OnPowserTurnEnded` (`self.PowserCharacter`) (delegate `StartTurn`)))

(event `StartTurn`
  (bind _output (`|GetArrayItem` (`self.RoundOrder`)))
  (`KismetSystemLibrary.Delay` 1.0)
  (set `/Game/W_Roll.RolledThisTurn` false (`/Game/BP_Character.As W Roll` _output))
  (`/Game/BP_Character.RollDice` _output)
  (add `/Game/BP_Character.OnTurnEnded` _output (delegate `NextTurn`)))

(event `NextTurn`
  (`KismetArrayLibrary.Array_Remove` (`self.RoundOrder`))
  (if (`KismetArrayLibrary.Array_IsEmpty` (`self.RoundOrder`))
    (`self.EndRound`)
    (else
      (`self.StartTurn`))))

(event `StartTurnPowser`
  (bind _powsercharacter (`self.PowserCharacter`))
  (`KismetSystemLibrary.Delay` 2.0)
  (set `/Game/W_Roll.RolledThisTurn` true (`/Game/BP_PowserCharacter.As W Powser` _powsercharacter))
  (`/Game/BP_PowserCharacter.OnTurn` _powsercharacter))

(fn `UserConstructionScript`)